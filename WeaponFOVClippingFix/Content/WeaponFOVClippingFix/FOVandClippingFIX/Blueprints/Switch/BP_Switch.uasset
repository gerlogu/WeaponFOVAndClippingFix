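; BP_Switch is a toggle switch that turns the fixed weapon mode on the player's FirstPersonCharacter on or off.
; Its Switch event flips IsActive, passes the state to SwitchFixedWeapon and shows or hides the Checker component to match.
; The construction script gives the Checker, four side pieces and text render dynamic materials tinted with a shared MaterialColor.
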(event `Event Switch`
  ;[0 0 0] Event Switch
  (set `self.IsActive` (not (`self.IsActive`)))
  (bind _asfirst_person_character (cast `/Game/WeaponFOVClippingFix/FOVandClippingFIX/Blueprints/Character/FirstPersonCharacter` (`GameplayStatics.GetPlayerCharacter` 0)))
  (`/Game/WeaponFOVClippingFix/FOVandClippingFIX/Blueprints/Character/FirstPersonCharacter.SwitchFixedWeapon` _asfirst_person_character (`self.IsActive`))
  (`SceneComponent.SetVisibility` (`self.Checker`) (`self.IsActive`) false))

(fn `SetMaterial`
  (params (Target :type "PrimitiveComponent Object Reference"))
  ;[0 0 0] Set Material
  (bind _returnvalue (`PrimitiveComponent.CreateDynamicMaterialInstance` Target 0 (`PrimitiveComponent.GetMaterial` Target 0) "None"))
  (`MaterialInstanceDynamic.SetVectorParameterValue` _returnvalue "Color" (`self.MaterialColor`)))

(fn `UserConstructionScript`
  ;[0 0 0] Construction Script
  (`self.SetMaterial` (`self.Checker`))
  (`self.SetMaterial` (`self.Left`))
  (`self.SetMaterial` (`self.Up`))
  (`self.SetMaterial` (`self.Down`))
  (`self.SetMaterial` (`self.Right`))
  (`self.SetMaterial` (`self.TextRender`)))