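; FPS movement sway component that rolls an assigned scene component in response to a movement input value.
; Init stores the component to move.
; CalculateSway scales MovementY by SwayAmount, clamps it to that range, and interpolates the component's relative roll toward it with FInterpTo and world delta time, leaving pitch and yaw unchanged.
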(fn `CalculateSway`
  (params (MovementY :type "Float (double-precision)"))
  (bind _relativerotation_roll (`KismetMathLibrary.BreakRotator` (`SceneComponent.RelativeRotation` (`self.ComponentToMove`))))
  (bind (_relativerotation_roll_2 _relativerotation_pitch _relativerotation_yaw) (`KismetMathLibrary.BreakRotator` (`SceneComponent.RelativeRotation` (`self.ComponentToMove`))))
  (`SceneComponent.K2_SetRelativeRotation` (`self.ComponentToMove`) (`KismetMathLibrary.MakeRotator` (`KismetMathLibrary.FInterpTo` _relativerotation_roll (`KismetMathLibrary.FClamp` (* MovementY (`self.SwayAmount`)) (* (`self.SwayAmount`) -1.0) (`self.SwayAmount`)) (`GameplayStatics.GetWorldDeltaSeconds`) (`self.InterpSpeed`)) _relativerotation_pitch _relativerotation_yaw) false false))

(fn `Init`
  (params (ComponentToMove :type "SceneComponent Object Reference"))
  ;[0 0 0] Init
  (set `self.ComponentToMove` ComponentToMove))