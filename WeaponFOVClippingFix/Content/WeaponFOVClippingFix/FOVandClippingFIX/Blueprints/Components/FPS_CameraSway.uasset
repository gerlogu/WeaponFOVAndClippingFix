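; FPS camera sway component that rotates a supplied component in response to X and Y axis input.
; Init stores the component to move, and CalculateSway scales both axes by LookAmount, clamping them through CheckLookAmount.
; X drives roll and yaw and Y drives inverted pitch as offsets from InitialRot.
; The relative rotation lerps toward that target using SmoothAmount times delta seconds.
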(fn `CalculateSway`
  (params (XAxis :type "Float (double-precision)") (YAxis :type "Float (double-precision)"))
  (returns (ReturnValue :type "Rotator Structure"))
  (bind _newammount (`self.CheckLookAmount` (* (`local.XAxis`) (`self.LookAmount`))))
  (bind _returnvalue (`KismetMathLibrary.RLerp` (`SceneComponent.RelativeRotation` (`self.ComponentToMove`)) (`KismetMathLibrary.MakeRotator` (+ (.roll (`self.InitialRot`)) (.roll (`KismetMathLibrary.MakeRotator` _newammount (`self.CheckLookAmount` (* (`local.YAxis`) (`self.LookAmount`))) _newammount))) (- (.pitch (`self.InitialRot`)) (.pitch (`KismetMathLibrary.MakeRotator` _newammount (`self.CheckLookAmount` (* (`local.YAxis`) (`self.LookAmount`))) _newammount))) (+ (.yaw (`self.InitialRot`)) (.yaw (`KismetMathLibrary.MakeRotator` _newammount (`self.CheckLookAmount` (* (`local.YAxis`) (`self.LookAmount`))) _newammount)))) (* (`self.SmoothAmount`) (`GameplayStatics.GetWorldDeltaSeconds`))))
  ;[0 0 0] Calculate Sway
  (`SceneComponent.K2_SetRelativeRotation` (`self.ComponentToMove`) _returnvalue false false)
  (return _returnvalue))

(fn `CheckLookAmount`
  (params (CurrentAmount :type "Float (double-precision)"))
  (returns (NewAmmount :type "Float (double-precision)"))
  (bind _amountcap (`self.AmountCap`))
  (bind _returnvalue (* _amountcap -1.0))
  ;[0 0 0] Check Look Amount
  (if (> CurrentAmount _amountcap)
    (return (`self.AmountCap`))
    (elif (< (`local.CurrentAmount`) _returnvalue)
      (return _returnvalue)
      (else
        (return (`local.CurrentAmount`))))))

(fn `Init`
  (params (ComponentToMove :type "SceneComponent Object Reference"))
  ;[0 0 0] Init
  (set `self.ComponentToMove` ComponentToMove))