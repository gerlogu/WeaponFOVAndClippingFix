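; In-world vertical slider actor that adjusts either the first-person camera FOV or the weapon FOV, depending on SliderType.
; BeginPlay places the target from the current FOV along the spline's two endpoints.
; While dragging, a looping timer line-traces from the player camera and clamps the hit height to the spline.
; Tick moves the knob toward that target at constant speed, applying the FOV and updating the readout as it moves.
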(event `self.ReceiveBeginPlay`
  (bind (_returnvalue_x _returnvalue_y _returnvalue_z) (`KismetMathLibrary.BreakVector` (`SplineComponent.GetLocationAtSplinePoint` (`self.Spline`) 1 "World")))
  (bind (_returnvalue_x_2 _returnvalue_y_2 _returnvalue_z_2) (`KismetMathLibrary.BreakVector` (`SplineComponent.GetLocationAtSplinePoint` (`self.Spline`) 0 "World")))
  (bind (_returnvalue_x_3 _returnvalue_y_3 _returnvalue_z_3) (`KismetMathLibrary.BreakVector` (`SceneComponent.K2_GetComponentLocation` (`self.Value`))))
  (bind (_returnvalue_x_4 _returnvalue_y_4 _returnvalue_z_4) (`KismetMathLibrary.BreakVector` (`SplineComponent.GetLocationAtSplinePoint` (`self.Spline`) 0 "World")))
  (bind (_returnvalue_x_5 _returnvalue_y_5 _returnvalue_z_5) (`KismetMathLibrary.BreakVector` (`SplineComponent.GetLocationAtSplinePoint` (`self.Spline`) 1 "World")))
  ;[0 0 0] Event Begin Play
  (set `self.SliderValue` _returnvalue_z_3)
  (switch `/Game/WeaponFOVClippingFix/FOVandClippingFIX/Blueprints/Slider/E_SliderType` (`self.SliderType`)
    (:`NewEnumerator0`
      ;;[0.3073 0.1857 0.09398] Camera FOV
      (bind _asfirst_person_character (cast `/Game/WeaponFOVClippingFix/FOVandClippingFIX/Blueprints/Character/FirstPersonCharacter` (`GameplayStatics.GetPlayerCharacter` 0)))
      (bind _fieldofview (`CameraComponent.FieldOfView` (`/Game/WeaponFOVClippingFix/FOVandClippingFIX/Blueprints/Character/FirstPersonCharacter.FirstPersonCamera` _asfirst_person_character)))
      (`TextRenderComponent.K2_SetText` (`self.TextRender1`) (`KismetTextLibrary.Conv_IntToText` (`KismetMathLibrary.Round` _fieldofview)))
      (set `self.SliderValue` (`KismetMathLibrary.MapRangeClamped` _fieldofview 75.0 120.0 _returnvalue_z_4 _returnvalue_z_5)))
    (:`NewEnumerator1`
      ;;[0.1296 0.2552 0.1256] Weapon FOV
      (bind _asfirst_person_character_2 (cast `/Game/WeaponFOVClippingFix/FOVandClippingFIX/Blueprints/Character/FirstPersonCharacter` (`GameplayStatics.GetPlayerCharacter` 0)))
      (bind _returnvalue (`MaterialInstanceDynamic.K2_GetScalarParameterValue` (`/Game/WeaponFOVClippingFix/FOVandClippingFIX/Blueprints/Character/FirstPersonCharacter.ArmsMaterial` _asfirst_person_character_2) "FOV"))
      (`TextRenderComponent.K2_SetText` (`self.TextRender1`) (`KismetTextLibrary.Conv_IntToText` (`KismetMathLibrary.Round` _returnvalue)))
      (set `self.SliderValue` (`KismetMathLibrary.MapRangeClamped` _returnvalue (`/Game/WeaponFOVClippingFix/FOVandClippingFIX/Blueprints/Character/FirstPersonCharacter.MinFOV` _asfirst_person_character_2) (`/Game/WeaponFOVClippingFix/FOVandClippingFIX/Blueprints/Character/FirstPersonCharacter.MaxFOV` _asfirst_person_character_2) _returnvalue_z_2 _returnvalue_z)))))

(event `self.ReceiveTick`
  (params (DeltaSeconds :type "Float (single-precision)"))
  (bind _returnvalue (`self.GetSliderValue`))
  (bind (_returnvalue_x _returnvalue_y _returnvalue_z) (`KismetMathLibrary.BreakVector` (`SceneComponent.K2_GetComponentLocation` (`self.Value`))))
  (bind (_returnvalue_x_2 _returnvalue_y_2 _returnvalue_z_2) (`KismetMathLibrary.BreakVector` (`SceneComponent.K2_GetComponentLocation` (`self.Value`))))
  ;[0 0 0] Event Tick
  (if (!= _returnvalue_z_2 (`self.SliderValue`))
    (`SceneComponent.K2_SetWorldLocation` (`self.Value`) (`KismetMathLibrary.MakeVector` _returnvalue_x _returnvalue_y (`KismetMathLibrary.FInterpTo_Constant` _returnvalue_z (`self.SliderValue`) (`GameplayStatics.GetWorldDeltaSeconds`) (`self.UpdateSpeed`))) false false)
    (switch `/Game/WeaponFOVClippingFix/FOVandClippingFIX/Blueprints/Slider/E_SliderType` (`self.SliderType`)
      (:`NewEnumerator0`
        ;;[0.1771 0.1273 0.04796] World FOV
        (bind _asfirst_person_character (cast `/Game/WeaponFOVClippingFix/FOVandClippingFIX/Blueprints/Character/FirstPersonCharacter` (`GameplayStatics.GetPlayerCharacter` 0)))
        (set `CameraComponent.FieldOfView` (`KismetMathLibrary.Conv_IntToDouble` _returnvalue) (`/Game/WeaponFOVClippingFix/FOVandClippingFIX/Blueprints/Character/FirstPersonCharacter.FirstPersonCamera` _asfirst_person_character))
        (`TextRenderComponent.K2_SetText` (`self.TextRender1`) (`KismetTextLibrary.Conv_IntToText` _returnvalue)))
      (:`NewEnumerator1`
        ;;[0.05447 0.1458 0.0372] Weapon FOV
        (bind _asfirst_person_character_2 (cast `/Game/WeaponFOVClippingFix/FOVandClippingFIX/Blueprints/Character/FirstPersonCharacter` (`GameplayStatics.GetPlayerCharacter` 0)))
        (bind _currentfov (`/Game/WeaponFOVClippingFix/FOVandClippingFIX/Blueprints/Character/FirstPersonCharacter.UpdateFOV` _asfirst_person_character_2 (`self.GetNormalizedSliderValue`)))
        (`TextRenderComponent.K2_SetText` (`self.TextRender1`) (`KismetTextLibrary.Conv_IntToText` (`KismetMathLibrary.Round` _currentfov)))))))

(event `Event StartDrag`
  ;[0 0 0] Event StartDrag
  (bind _returnvalue (`KismetSystemLibrary.K2_SetTimerDelegate` (`|CreateDelegate` :!event `Event SetSliderValue`) 0.01 true))
  (set `self.SliderTimer` _returnvalue))

(event `Event EndDrag`
  ;[0 0 0] Event EndDrag
  (`KismetSystemLibrary.K2_ClearAndInvalidateTimerHandle` (`self.SliderTimer`)))

(event `Event SetSliderValue`
  (bind (_returnvalue_x _returnvalue_y _returnvalue_z) (`KismetMathLibrary.BreakVector` (`SplineComponent.GetLocationAtSplinePoint` (`self.Spline`) 1 "World")))
  (bind (_returnvalue_x_2 _returnvalue_y_2 _returnvalue_z_2) (`KismetMathLibrary.BreakVector` (`SplineComponent.GetLocationAtSplinePoint` (`self.Spline`) 0 "World")))
  ;[0 0 0] Event SetSliderValue
  (bind _asfirst_person_character (cast `/Game/WeaponFOVClippingFix/FOVandClippingFIX/Blueprints/Character/FirstPersonCharacter` (`GameplayStatics.GetPlayerCharacter` 0)))
  (bind _firstpersoncamera (`/Game/WeaponFOVClippingFix/FOVandClippingFIX/Blueprints/Character/FirstPersonCharacter.FirstPersonCamera` _asfirst_person_character))
  (bind (_outhit _returnvalue) (`KismetSystemLibrary.LineTraceSingle` :`Start` (`SceneComponent.K2_GetComponentLocation` _firstpersoncamera) :`End` (+ (`SceneComponent.K2_GetComponentLocation` _firstpersoncamera) (* (`SceneComponent.GetForwardVector` _firstpersoncamera) 1750.0)) :`TraceChannel` "TraceTypeQuery1" :`bIgnoreSelf` false))
  (if _returnvalue
    (set `self.SliderValue` (`KismetMathLibrary.FClamp` (.z (`.Location` (`GameplayStatics.BreakHitResult` _outhit))) _returnvalue_z_2 _returnvalue_z))))

(fn `GetNormalizedSliderValue`
  (returns (ReturnValue :type "Float (double-precision)"))
  (bind (_relativelocation_x _relativelocation_y _relativelocation_z) (`KismetMathLibrary.BreakVector` (`SceneComponent.RelativeLocation` (`self.Value`))))
  ;[0 0 0] Get Normalized Slider Value
  (return (`KismetMathLibrary.MapRangeClamped` _relativelocation_z -162.0 162.0 0.0 1.0)))

(fn `GetSliderValue`
  (returns (ReturnValue :type Integer))
  ;[0 0 0] Get Slider Value
  (bind (_minvalue _maxvalue) (`/Game/WeaponFOVClippingFix/FOVandClippingFIX/Blueprints/MacroLibraries/ML_FOV.GetWeaponFOVLimits`))
  (return (`KismetMathLibrary.Round` (`KismetMathLibrary.MapRangeClamped` (`self.GetNormalizedSliderValue`) 0.0 1.0 _minvalue _maxvalue))))

(fn `SetMaterial`
  (params (Target :type "PrimitiveComponent Object Reference"))
  ;[0 0 0] Set Material
  (bind _returnvalue (`PrimitiveComponent.CreateDynamicMaterialInstance` Target 0 (`PrimitiveComponent.GetMaterial` Target 0) "None"))
  (`MaterialInstanceDynamic.SetVectorParameterValue` _returnvalue "Color" (`self.MaterialColor`)))

(fn `UserConstructionScript`
  (`TextRenderComponent.K2_SetText` (`self.TextRender`) (`self.SliderName`))
  (`self.SetMaterial` (`self.Value`))
  (`self.SetMaterial` (`self.Top`))
  (`self.SetMaterial` (`self.Top`))
  (`self.SetMaterial` (`self.Bottom`))
  (`self.SetMaterial` (`self.TextRender1`))
  (`self.SetMaterial` (`self.TextRender`)))